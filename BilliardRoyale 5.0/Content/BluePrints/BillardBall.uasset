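; Billiard ball actor that plays a random 2D impact sound when its sphere hits another ball.
; Hits from player balls and from other billiard balls draw on separate sound sets, each gated by a DoOnce.
; Tick-driven Delays periodically reset the gates to throttle repeats, more slowly for billiard-ball hits.
; The billiard-ball gate starts closed, so those sounds are silent until its first reset.
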(event `self.Sphere.OnComponentHit`
  (params (HitComponent :type "PrimitiveComponent Object Reference") (OtherActor :type "Actor Object Reference") (OtherComp :type "PrimitiveComponent Object Reference") (NormalImpulse :type "Vector Structure") (Hit :type "HitResult Structure (by ref)"))
  ;[1 1 1] Plays sound on hit with player balls
  (`|ExecutionSequence`
    (:`then_0`
      (cast `/Game/BluePrints/PlayerBallActor` OtherActor)
      (`/Engine/EditorBlueprintResources/StandardMacros.DoOnce` false :!label _label
        (:`Completed`
          (`GameplayStatics.PlaySound2D` (`KismetArrayLibrary.Array_Random` (`|MakeArray` "/Game/Sounds-Music/Hit2_Cue.Hit2_Cue" "/Game/Sounds-Music/Hit5_Cue.Hit5_Cue" "/Game/Sounds-Music/Hit2.Hit2" "/Game/Sounds-Music/Hit5.Hit5" :!type "SoundBase Object Reference")) 1.0 1.0 0.0 null null))))
    (:`then_1`
      (cast `/Game/BluePrints/BillardBall` OtherActor)
      (`/Engine/EditorBlueprintResources/StandardMacros.DoOnce` true :!label _label_2
        (:`Completed`
          (`GameplayStatics.PlaySound2D` (`KismetArrayLibrary.Array_Random` (`|MakeArray` "/Game/Sounds-Music/Hit1_Cue.Hit1_Cue" "/Game/Sounds-Music/Hit3_Cue.Hit3_Cue" "/Game/Sounds-Music/Hit4_Cue.Hit4_Cue" :!type "SoundBase Object Reference")) 1.0 1.0 0.0 null null))))))

(event `self.ReceiveTick`
  (params (DeltaSeconds :type "Float (single-precision)"))
  ;[1 1 1] Plays sound on hit with player balls
  (`KismetSystemLibrary.Delay` 1.0)
  (`|ExecutionSequence`
    (:`then_0`
      (goto _label :!via `Reset`))
    (:`then_1`
      (`KismetSystemLibrary.Delay` 2.0)
      (goto _label_2 :!via `Reset`))))

(fn `UserConstructionScript`)